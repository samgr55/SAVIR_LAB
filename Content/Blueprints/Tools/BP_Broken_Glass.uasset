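; BP_Broken_Glass is a trigger actor for broken glass that draws the player's attention and shows an info widget.
; When a ThirdPersonCharacter overlaps its Sphere, the character's controller rotation snaps to face the actor.
; The widget from its GeneralInfoWidgetComponent becomes visible, then collapses after a five-second delay.
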(event `self.Sphere.OnComponentBeginOverlap`
  (params (OverlappedComponent :type "PrimitiveComponent Object Reference") (OtherActor :type "Actor Object Reference") (OtherComp :type "PrimitiveComponent Object Reference") (OtherBodyIndex :type Integer) (bFromSweep :type Boolean) (SweepResult :type "HitResult Structure (by ref)"))
  (bind _returnvalue (`WidgetComponent.GetWidget` (`self.GetComponentByClass` self "/Script/SAVIR_Labs.GeneralInfoWidgetComponent")))
  (bind _asthird_person_character (cast `/Game/ThirdPersonBP/Blueprints/ThirdPersonCharacter` OtherActor))
  (`Controller.SetControlRotation` (`Pawn.GetController` _asthird_person_character) (`KismetMathLibrary.FindLookAtRotation` (`self.K2_GetActorLocation` _asthird_person_character) (`self.K2_GetActorLocation` self)))
  (`Widget.SetVisibility` _returnvalue "Visible")
  (`KismetSystemLibrary.Delay` 5.0)
  (`Widget.SetVisibility` _returnvalue "Collapsed"))

(fn `UserConstructionScript`)