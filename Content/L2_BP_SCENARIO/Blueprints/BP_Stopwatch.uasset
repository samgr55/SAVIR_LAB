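; BP_Stopwatch is the input layer for a player-operated stopwatch and a diffusion data entry screen.
; Input actions forward start/stop, reset, register time and clear time table commands to WatchWidget while it is in the viewport.
; EnterData toggles DiffusionDataEntryWidget, opening only while the watch is shown, with the cursor visible and move and look input ignored until it closes.
; Neither widget is created in these graphs.
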(event `InputAction|StartTime`
  (params (Key :type "Key Structure"))
  (bind _watchwidget (`self.WatchWidget`))
  ;[1 1 1] Start/Stop Timer
  (:`Pressed`
    (if (`Widget.IsInViewport` _watchwidget)
      (`WatchWidget.TrackTime` _watchwidget))))

(event `InputAction|EnterData` :consume false
  (params (Key :type "Key Structure"))
  (bind _returnvalue (`GameplayStatics.GetPlayerController` 0))
  (bind _returnvalue_2 (`GameplayStatics.GetPlayerController` 0))
  (bind _diffusiondataentrywidget (`self.DiffusionDataEntryWidget`))
  ;[1 1 1] EnterData
  (:`Pressed`
    (if (and (`Widget.IsInViewport` (`self.WatchWidget`)) (not (`Widget.IsInViewport` _diffusiondataentrywidget)))
      (`UserWidget.AddToViewport` _diffusiondataentrywidget 0)
      ;[1 1 1] Show/Hide Mouse
      (set `PlayerController.bShowMouseCursor` true _returnvalue_2)
      (`Controller.SetIgnoreMoveInput` _returnvalue_2 true)
      (`Controller.SetIgnoreLookInput` _returnvalue true)
      (else
        (`Widget.RemoveFromParent` _diffusiondataentrywidget)
        (set `PlayerController.bShowMouseCursor` false _returnvalue)
        (`Controller.SetIgnoreMoveInput` _returnvalue false)
        (`Controller.SetIgnoreLookInput` _returnvalue false)))))

(event `InputAction|ResetTime`
  (params (Key :type "Key Structure"))
  (bind _watchwidget (`self.WatchWidget`))
  ;[1 1 1] ResetTimer
  (:`Pressed`
    (if (`Widget.IsInViewport` _watchwidget)
      (`WatchWidget.ResetTimer` _watchwidget))))

(event `InputAction|ClearTimeTable`
  (params (Key :type "Key Structure"))
  (bind _watchwidget (`self.WatchWidget`))
  ;[1 1 1] ResetTimerTable
  (:`Pressed`
    (if (`Widget.IsInViewport` _watchwidget)
      (`WatchWidget.ResetRegisteredTime` _watchwidget))))

(event `InputAction|EnterInTmeTable`
  (params (Key :type "Key Structure"))
  (bind _watchwidget (`self.WatchWidget`))
  ;[1 1 1] RegisterTimeTable
  (:`Pressed`
    (if (`Widget.IsInViewport` _watchwidget)
      (`WatchWidget.RegisterTime` _watchwidget))))

(fn `UserConstructionScript`)